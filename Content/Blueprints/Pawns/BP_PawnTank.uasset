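; BP_PawnTank is a tank pawn Blueprint that shows its health on an on-screen HUD.
; On BeginPlay it creates the WBP_PlayerHealth widget, adds it to the viewport and initializes it from HealthComponent's current and default health.
; On AnyDamage it refreshes the widget with current health minus a hardcoded amount rather than the event's damage value, leaving HealthComponent itself untouched.
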(event EventBeginPlay
  (bind _healthcomponent (Variables|Default|GetHealthComponent))
  (bind _returnvalue (UserInterface|CreateWidget "/Game/Blueprints/Widgets/WBP_PlayerHealth.WBP_PlayerHealth_C"))
  (bind _output_get (Variables|Default|SetHUDdRef _returnvalue))
  (UserInterface|Viewport|AddtoViewport _output_get 0)
  (Default|UpdateHealth (Variables|Default|GetHUDdRef) (Variables|/Script/ToonTanks.HealthComponent|GetHealth _healthcomponent) (Variables|/Script/ToonTanks.HealthComponent|GetDefaultHealth _healthcomponent)))

(event Game|Damage|EventAnyDamage
  (params (Damage :type Float%20%28single-precision%29) (DamageType :type Damage%20Type%20Object%20Reference) (InstigatedBy :type Controller%20Object%20Reference) (DamageCauser :type Actor%20Object%20Reference))
  (bind _healthcomponent (Variables|Default|GetHealthComponent))
  (bind _huddref (Variables|Default|GetHUDdRef))
  (Utilities|IsValid _huddref
    (:Is%20Valid
      (Default|UpdateHealth _huddref (- (Variables|/Script/ToonTanks.HealthComponent|GetHealth _healthcomponent) 25.0) (Variables|/Script/ToonTanks.HealthComponent|GetDefaultHealth _healthcomponent)))))

(fn ConstructionScript)