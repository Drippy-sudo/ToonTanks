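; BP_PawnTurret is a turret pawn Blueprint that drives an enemy health bar widget.
; On BeginPlay it casts the HealthBar component's widget to WBP_EnemyHealthBar, caches it and initializes it from HealthComponent's current and default health.
; AnyDamage refreshes the bar with current health minus a hard-coded amount, ignoring the actual damage value and leaving HealthComponent unchanged in this graph.
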(event EventBeginPlay
  (bind _healthcomponent (Variables|Default|GetHealthComponent))
  (bind _aswbp_enemy_health_bar (Utilities|Casting|CastToWBP_EnemyHealthBar (UserInterface|GetUserWidgetObject (Variables|Default|GetHealthBar))))
  (bind _output_get (Variables|Default|SetEnemyHPWidget _aswbp_enemy_health_bar))
  (Default|UpdateHealth _output_get (Variables|/Script/ToonTanks.HealthComponent|GetHealth _healthcomponent) (Variables|/Script/ToonTanks.HealthComponent|GetDefaultHealth _healthcomponent)))

(event Game|Damage|EventAnyDamage
  (params (Damage :type Float%20%28single-precision%29) (DamageType :type Damage%20Type%20Object%20Reference) (InstigatedBy :type Controller%20Object%20Reference) (DamageCauser :type Actor%20Object%20Reference))
  (bind _healthcomponent (Variables|Default|GetHealthComponent))
  (Default|UpdateHealth (Variables|Default|GetEnemyHPWidget) (- (Variables|/Script/ToonTanks.HealthComponent|GetHealth _healthcomponent) 25.0) (Variables|/Script/ToonTanks.HealthComponent|GetDefaultHealth _healthcomponent)))

(fn ConstructionScript)