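; BP_GameModeBase is a game mode Blueprint that drives the start, score and game-over UI.
; GameStart creates and shows the start widget, passing it StartDelay, along with a score widget that Tick updates from Score every frame.
; GameOver creates and shows the end widget, passing PlayerWon through a setter named SetStartDelay.
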(event EventTick
  (params (DeltaSeconds :type Float%20%28single-precision%29))
  (Default|SetScore (stale EventGameStart _returnvalue_2) (Variables|Default|GetScore)))

(event EventGameStart
  (bind _returnvalue (UserInterface|CreateWidget "/Game/Blueprints/Widgets/WBP_GameStart.WBP_GameStart_C"))
  (Default|SetStartDelay _returnvalue (Variables|Default|GetStartDelay))
  (bind _returnvalue_2 (UserInterface|CreateWidget "/Game/Blueprints/Widgets/WBP_Score.WBP_Score_C"))
  (UserInterface|Viewport|AddtoViewport _returnvalue 0))

(event EventGameOver
  (params (PlayerWon :type Boolean))
  (bind _returnvalue (UserInterface|CreateWidget "/Game/Blueprints/Widgets/WBP_GameEnd.WBP_GameEnd_C"))
  (Default|SetStartDelay _returnvalue PlayerWon)
  (UserInterface|Viewport|AddtoViewport _returnvalue 0))

(fn ConstructionScript)